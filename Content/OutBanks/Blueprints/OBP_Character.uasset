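; OBP_Character is a character Blueprint that drives the player's HUD.
; It creates BP_HUDWidget on BeginPlay, and events push ammo, weapon name and health values from AmmoComp, WeaponHandle and HealthComp into the widget's variables.
; Tick also writes a distance readout each frame, derived from the actor's world X position scaled down and floored.
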(event `self.ReceiveBeginPlay`
  (bind _returnvalue (`|CreateWidget` "/Game/OutBanks/Blueprints/BP_HUDWidget.BP_HUDWidget_C"))
  (bind _output_get (set `self.HUDWidget` _returnvalue))
  (`UserWidget.AddToViewport` _output_get 0))

(event `self.UpdateAmmoHUD`
  (bind _ammocomp (`self.AmmoComp`))
  (bind _hudwidget (`self.HUDWidget`))
  (set `/Game/OutBanks/Blueprints/BP_HUDWidget.AmmoInReserve` (`OB_AmmoComp.CurrentAmmoInReserve` _ammocomp) _hudwidget)
  (set `/Game/OutBanks/Blueprints/BP_HUDWidget.CurrentAmmo` (`OB_AmmoComp.CurrentAmmoInClip` _ammocomp) _hudwidget))

(event `self.OnPickUpWeaponUpdateHUD`
  (set `/Game/OutBanks/Blueprints/BP_HUDWidget.MaxAmmo` (`OB_AmmoComp.MaxAmmoInClip` (`self.AmmoComp`)) (`self.HUDWidget`))
  (set `/Game/OutBanks/Blueprints/BP_HUDWidget.WeaponName` (`KismetTextLibrary.Conv_NameToText` (`OB_WeaponBase.WeaponName` (`self.WeaponHandle`))) (`self.HUDWidget`)))

(event `self.UpdateHealthHUD`
  (bind _returnvalue (`OB_HealthComp.GetHealthPercent` (`self.HealthComp`)))
  (set `/Game/OutBanks/Blueprints/BP_HUDWidget.LifePercent` _returnvalue (`self.HUDWidget`)))

(event `self.ReceiveTick`
  (params (DeltaSeconds :type "Float (single-precision)"))
  (bind _returnvalue_x (`KismetMathLibrary.BreakVector` (`self.K2_GetActorLocation`)))
  (set `/Game/OutBanks/Blueprints/BP_HUDWidget.Distance` (`KismetMathLibrary.FFloor` (/ _returnvalue_x 100.0)) (`self.HUDWidget`)))

(fn `UserConstructionScript`)